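; Draggable actor that tracks the BP_Location and BP_Fire it overlaps and can be burned; the dragging logic itself is not here.
; Cube overlap events set and clear both references, which Tick prints as debug text.
; Burn attaches a fire particle, disables collision, and uses a timeline to lerp the actor to just above the first BP_Fire in the level while zeroing its rotation, then destroys it.
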(event OnComponentBeginOverlap(Cube)
  (params (OverlappedComponent :type Primitive%20Component%20Object%20Reference) (OtherActor :type Actor%20Object%20Reference) (OtherComp :type Primitive%20Component%20Object%20Reference) (OtherBodyIndex :type Integer) (bFromSweep :type Boolean) (SweepResult :type Hit%20Result%20Structure%20%28by%20ref%29))
  (bind _asbp_location (Utilities|Casting|CastToBP_Location OtherActor)
    (:then
      (Variables|Default|SetLocation _asbp_location))
    (:CastFailed
      (bind _asbp_fire (Utilities|Casting|CastToBP_Fire OtherActor))
      (Variables|Default|SetFire _asbp_fire))))

(event OnComponentEndOverlap(Cube)
  (params (OverlappedComponent :type Primitive%20Component%20Object%20Reference) (OtherActor :type Actor%20Object%20Reference) (OtherComp :type Primitive%20Component%20Object%20Reference) (OtherBodyIndex :type Integer))
  (Utilities|Casting|CastToBP_Location OtherActor
    (:then
      (Variables|Default|SetLocation 0))
    (:CastFailed
      (Utilities|Casting|CastToBP_Fire OtherActor)
      (Variables|Default|SetFire 0))))

(event Custom|Burn
  (bind _cube (Variables|Default|GetCube))
  (bind _returnvalue (AddComponent|AddParticleSystemComponent false (Math|Transform|MakeTransform "0, 0, 0" "0, 0, 0" "5.000000,5.000000,5.000000")))
  (Effects|Components|ParticleSystem|SetTemplate _returnvalue "/Game/StarterContent/Particles/P_Fire.P_Fire")
  (Collision|SetCollisionEnabled (Variables|Default|GetCube) "NoCollision")
  (bind _output_get (Variables|Default|SetEndobjectlocation (Transformation|GetActorLocation)))
  (bind _output_get_2 (Variables|Default|Setendobjectrotation (Transformation|GetActorRotation)))
  (bind _outactors (Actor|GetAllActorsOfClass "/Game/StarterContent/Blueprints/BP_Fire.BP_Fire_C"))
  (bind _newtrack_0 (Timeline|Timeline_0 PlayFromStart)
    (:Update
      (Transformation|SetActorLocation (Math|Vector|Lerp(Vector) _output_get (+ (Transformation|GetActorLocation (Utilities|Array|Get(acopy) _outactors)) "0, 0,10.000000") _newtrack_0) false false)
      (Transformation|SetActorRotation (Math|Rotator|Lerp(Rotator) _output_get_2 "0, 0, 0" _newtrack_0)))
    (:Finished
      (Collision|SetCollisionEnabled _cube "QueryAndPhysics")
      (Collision|SetCollisionResponsetoChannel _cube "ECC_Visibility" "ECR_Block")
      (Collision|SetCollisionResponsetoChannel _cube "ECC_Camera" "ECR_Block")
      (Actor|DestroyActor))))

(event EventBeginPlay
  (bind _outactors (Actor|GetAllActorsOfClass "/Game/Camera/Camera.Camera_C"))
  (Variables|Default|SetCamera (Utilities|Array|Get(acopy) _outactors)))

(event EventTick
  (params (DeltaSeconds :type Float%20%28single-precision%29))
  (Development|PrintString (Utilities|GetObjectName (Variables|Default|GetLocation)) true true "(R=0.000000,G=0.660000,B=1.000000,A=1.000000)" DeltaSeconds)
  (Development|PrintString (Utilities|GetObjectName (Variables|Default|GetFire)) true true "(R=0.000000,G=0.660000,B=1.000000,A=1.000000)" DeltaSeconds))

(fn ConstructionScript)