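; BP_Resource defines the game's resource types (Wood, Stone, Hydrogen, Cloth and Radus) and starting player inventory data for them.
; On BeginPlay it fills two hardcoded struct arrays: DataResources, which sets each resource's effect on fuel, and DataPlayer, which starts every inventory total at zero.
; It only initializes this data, with no other logic and an empty construction script.
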(event EventBeginPlay
  (Variables|Default|SetData_Resources (Utilities|Array|MakeArray (Utilities|Struct|MakeData_Resources "Wood" 6) (Utilities|Struct|MakeData_Resources "Stone") (Utilities|Struct|MakeData_Resources "Hydrogen" -1) (Utilities|Struct|MakeData_Resources "Cloth" 1) (Utilities|Struct|MakeData_Resources "Radus" 1)))
  (Variables|Default|SetData_Player (Utilities|Array|MakeArray (Utilities|Struct|MakeData_Player "Wood") (Utilities|Struct|MakeData_Player "Stone") (Utilities|Struct|MakeData_Player "Hydrogen") (Utilities|Struct|MakeData_Player "Cloth") (Utilities|Struct|MakeData_Player "Radus"))))

(fn ConstructionScript)