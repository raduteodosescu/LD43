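; Bowling centre location that, when staffed by a survivor, yields resources from its limited stock into the shared BP_Resource inventory.
; On BeginPlay with a survivor assigned, a short delay precedes five ProduceRaduce calls, each crediting a product and lowering its remaining amount.
; RemoveSurvivor then returns the survivor to inventory slot 0 and clears the flag.
; AddSurvivor and the random bonus UpgradeProduction are defined, but their event-graph calls never run.
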(event EventBeginPlay
  (if (Variables|Default|GetItHasSurvivor)
    (Utilities|FlowControl|RetriggerableDelay 0.1)
    (Utilities|FlowControl|Sequence
      (:then_0
        (bind _amount_left (CallFunction|Produce&Raduce (Variables|Products|GetPC1) (Variables|Products|GetPA1) (Variables|Products|GetTA1)))
        (Variables|Products|SetTA1 _amount_left))
      (:then_1
        (bind _amount_left_2 (CallFunction|Produce&Raduce (Variables|Products|GetPC1_0) (Variables|Products|GetPA1_0) (Variables|Products|GetTA1_0)))
        (Variables|Products|SetTA1_0 _amount_left_2))
      (:then_2
        (bind _amount_left_3 (CallFunction|Produce&Raduce (Variables|Products|GetPC1_1) (Variables|Products|GetPA1_1) (Variables|Products|GetTA1_1)))
        (Variables|Products|SetTA1_1 _amount_left_3))
      (:then_3
        (bind _amount_left_4 (CallFunction|Produce&Raduce (Variables|Products|GetPC1_2) (Variables|Products|GetPA1_2) (Variables|Products|GetTA1_2)))
        (Variables|Products|SetTA1_2 _amount_left_4))
      (:then_4
        (bind _amount_left_5 (CallFunction|Produce&Raduce (Variables|Products|GetPC1_3) (Variables|Products|GetPA1_3) (Variables|Products|GetTA1_3)))
        (Variables|Products|SetTA1_3 _amount_left_5))
      (:then_5
        (CallFunction|RemoveSurvivor)))))

(fn ConstructionScript)

(fn Produce&Raduce
  (params (Product :type Integer) (Produce :type Integer) (AmountLeft :type Integer))
  (if (<= AmountLeft 0)
    (return 0)
    (else
      (LocalVariables|SetProductCode Product)
      (LocalVariables|SetProduceAmount Produce)
      (LocalVariables|SetAmountLeftTotal AmountLeft)
      (LocalVariables|SetAmountLeftTotal (- (LocalVariables|GetAmountLeftTotal) (LocalVariables|GetProduceAmount)))
      (bind _outactors (Actor|GetAllActorsOfClass "/Game/Machinations/resources/BP_Resource.BP_Resource_C"))
      (Utilities|Array|SetArrayElem (Variables|/Game/Machinations/resources/BP_Resource.BP_Resource_C|GetData_Resources (Utilities|Array|Get(acopy) _outactors)) (LocalVariables|GetProductCode) (Utilities|Struct|MakeData_Resources "None" 0 (+ (.InInventory (Utilities|Struct|BreakData_Resources (Utilities|Array|Get(acopy) (Variables|/Game/Machinations/resources/BP_Resource.BP_Resource_C|GetData_Resources (Utilities|Array|Get(acopy) _outactors)) (LocalVariables|GetProductCode)))) (LocalVariables|GetProduceAmount)) 0))
      (Utilities|Struct|SetmembersinData_Production (Utilities|Struct|MakeData_Production (Utilities|Array|Get(acopy) (Variables|/Game/Machinations/resources/BP_Resource.BP_Resource_C|GetData_Resources (Utilities|Array|Get(acopy) _outactors)) (LocalVariables|GetProductCode)) (LocalVariables|GetAmountLeftTotal) (LocalVariables|GetProduceAmount)))
      (return (LocalVariables|GetAmountLeftTotal)))))

(fn UpgradeProduction
  (params (Product :type Integer) (Chance :type Integer))
  (LocalVariables|SetProductCode Product)
  (bind _outactors (Actor|GetAllActorsOfClass "/Game/Machinations/resources/BP_Resource.BP_Resource_C"))
  (if (<= (Math|Random|RandomIntegerinRange Chance 100) 0)
    (Utilities|Struct|SetmembersinData_Production (Utilities|Struct|MakeData_Production (Utilities|Array|Get(acopy) (Variables|/Game/Machinations/resources/BP_Resource.BP_Resource_C|GetData_Resources (Utilities|Array|Get(acopy) _outactors)) (LocalVariables|GetProductCode))))
    (Utilities|Array|SetArrayElem (Variables|/Game/Machinations/resources/BP_Resource.BP_Resource_C|GetData_Resources (Utilities|Array|Get(acopy) _outactors)) 0 (Utilities|Struct|MakeData_Resources "None" 0 (+ (.InInventory (Utilities|Struct|BreakData_Resources (Utilities|Array|Get(acopy) (Variables|/Game/Machinations/resources/BP_Resource.BP_Resource_C|GetData_Resources (Utilities|Array|Get(acopy) _outactors)) (LocalVariables|GetProductCode)))) 1) 0)))
  (return))

(fn AddSurvivor
  (bind _outactors (Actor|GetAllActorsOfClass "/Game/Machinations/resources/BP_Resource.BP_Resource_C"))
  (if (== (.InInventory (Utilities|Struct|BreakData_Resources (Utilities|Array|Get(acopy) (Variables|/Game/Machinations/resources/BP_Resource.BP_Resource_C|GetData_Resources (Utilities|Array|Get(acopy) _outactors))))) 0)
    _
    (else
      (Variables|Default|SetItHasSurvivor true)
      (Utilities|Array|SetArrayElem (Variables|/Game/Machinations/resources/BP_Resource.BP_Resource_C|GetData_Resources (Utilities|Array|Get(acopy) _outactors)) 0 (Utilities|Struct|MakeData_Resources "None" 0 (- (.InInventory (Utilities|Struct|BreakData_Resources (Utilities|Array|Get(acopy) (Variables|/Game/Machinations/resources/BP_Resource.BP_Resource_C|GetData_Resources (Utilities|Array|Get(acopy) _outactors))))) 1) 0))))
  (return))

(fn RemoveSurvivor
  (bind _outactors (Actor|GetAllActorsOfClass "/Game/Machinations/resources/BP_Resource.BP_Resource_C"))
  (Utilities|Array|SetArrayElem (Variables|/Game/Machinations/resources/BP_Resource.BP_Resource_C|GetData_Resources (Utilities|Array|Get(acopy) _outactors)) 0 (Utilities|Struct|MakeData_Resources "None" 0 (+ (.InInventory (Utilities|Struct|BreakData_Resources (Utilities|Array|Get(acopy) (Variables|/Game/Machinations/resources/BP_Resource.BP_Resource_C|GetData_Resources (Utilities|Array|Get(acopy) _outactors))))) 1) 0))
  (Variables|Default|SetItHasSurvivor false)
  (return))