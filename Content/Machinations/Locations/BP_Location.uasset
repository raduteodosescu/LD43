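; BP_Location is a resource site that a survivor works, draining its finite supply into the inventory held by the first BP_Resource actor.
; On BeginPlay, if occupied, it waits briefly, runs ProduceRaduce, rolls UpgradeProduction for a bonus item, then RemoveSurvivor returns the survivor.
; AddSurvivor takes a survivor from inventory, but its call in the event graph never runs.
; Tick prints the remaining supply for debugging.
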(event EventBeginPlay
  (if (Variables|Default|GetItHasSurvivor)
    (Utilities|FlowControl|RetriggerableDelay 0.1)
    (Utilities|FlowControl|Sequence
      (:then_0
        (bind _amount_left (CallFunction|Produce&Raduce (Variables|Default|GetResource1ProductCode) (Variables|Default|GetResource1ProduceTick) (Variables|Default|GetResource1TotalAmount)))
        (bind _output_get (Variables|Default|SetResource1TotalAmount _amount_left)))
      (:then_1
        (CallFunction|UpgradeProduction (Variables|Default|GetUpgrade1ProductCode) (Variables|Default|GetUpgrade1ProductChance)))
      (:then_2
        (CallFunction|RemoveSurvivor)))))

(event EventTick
  (params (DeltaSeconds :type Float%20%28single-precision%29))
  (Development|PrintString (Utilities|String|ToString(Float) (Math|Conversions|ToFloat(Integer) (stale EventBeginPlay _output_get))) true true "(R=0.000000,G=0.660000,B=1.000000,A=1.000000)" DeltaSeconds))

(fn ConstructionScript)

(fn Produce&Raduce
  (params (Product :type Integer) (Produce :type Integer) (AmountLeft :type Integer))
  (if (<= AmountLeft 0)
    (return 0)
    (else
      (LocalVariables|SetProductCode Product)
      (LocalVariables|SetProduceAmount Produce)
      (LocalVariables|SetAmountLeftTotal AmountLeft)
      (LocalVariables|SetAmountLeftTotal (- (LocalVariables|GetAmountLeftTotal) (LocalVariables|GetProduceAmount)))
      (bind _outactors (Actor|GetAllActorsOfClass "/Game/Machinations/resources/BP_Resource.BP_Resource_C"))
      (Utilities|Array|SetArrayElem (Variables|/Game/Machinations/resources/BP_Resource.BP_Resource_C|GetData_Resources (Utilities|Array|Get(acopy) _outactors)) (LocalVariables|GetProductCode) (Utilities|Struct|MakeData_Resources "None" 0 (+ (.InInventory (Utilities|Struct|BreakData_Resources (Utilities|Array|Get(acopy) (Variables|/Game/Machinations/resources/BP_Resource.BP_Resource_C|GetData_Resources (Utilities|Array|Get(acopy) _outactors)) (LocalVariables|GetProductCode)))) (LocalVariables|GetProduceAmount)) 0))
      (Utilities|Struct|SetmembersinData_Production (Utilities|Struct|MakeData_Production (Utilities|Array|Get(acopy) (Variables|/Game/Machinations/resources/BP_Resource.BP_Resource_C|GetData_Resources (Utilities|Array|Get(acopy) _outactors)) (LocalVariables|GetProductCode)) (LocalVariables|GetAmountLeftTotal) (LocalVariables|GetProduceAmount)))
      (return (LocalVariables|GetAmountLeftTotal)))))

(fn UpgradeProduction
  (params (Product :type Integer) (Chance :type Integer))
  (LocalVariables|SetProductCode Product)
  (bind _outactors (Actor|GetAllActorsOfClass "/Game/Machinations/resources/BP_Resource.BP_Resource_C"))
  (if (<= (Math|Random|RandomIntegerinRange Chance 100) 0)
    (Utilities|Struct|SetmembersinData_Production (Utilities|Struct|MakeData_Production (Utilities|Array|Get(acopy) (Variables|/Game/Machinations/resources/BP_Resource.BP_Resource_C|GetData_Resources (Utilities|Array|Get(acopy) _outactors)) (LocalVariables|GetProductCode))))
    (Utilities|Array|SetArrayElem (Variables|/Game/Machinations/resources/BP_Resource.BP_Resource_C|GetData_Resources (Utilities|Array|Get(acopy) _outactors)) 0 (Utilities|Struct|MakeData_Resources "None" 0 (+ (.InInventory (Utilities|Struct|BreakData_Resources (Utilities|Array|Get(acopy) (Variables|/Game/Machinations/resources/BP_Resource.BP_Resource_C|GetData_Resources (Utilities|Array|Get(acopy) _outactors)) (LocalVariables|GetProductCode)))) 1) 0)))
  (return))

(fn AddSurvivor
  (bind _outactors (Actor|GetAllActorsOfClass "/Game/Machinations/resources/BP_Resource.BP_Resource_C"))
  (if (== (.InInventory (Utilities|Struct|BreakData_Resources (Utilities|Array|Get(acopy) (Variables|/Game/Machinations/resources/BP_Resource.BP_Resource_C|GetData_Resources (Utilities|Array|Get(acopy) _outactors)) (Variables|Default|GetSurvivorCode)))) 0)
    _
    (else
      (Variables|Default|SetItHasSurvivor true)
      (Utilities|Array|SetArrayElem (Variables|/Game/Machinations/resources/BP_Resource.BP_Resource_C|GetData_Resources (Utilities|Array|Get(acopy) _outactors)) (Variables|Default|GetSurvivorCode) (Utilities|Struct|MakeData_Resources "None" 0 (- (.InInventory (Utilities|Struct|BreakData_Resources (Utilities|Array|Get(acopy) (Variables|/Game/Machinations/resources/BP_Resource.BP_Resource_C|GetData_Resources (Utilities|Array|Get(acopy) _outactors)) (Variables|Default|GetSurvivorCode)))) 1) 0))))
  (return))

(fn RemoveSurvivor
  (bind _outactors (Actor|GetAllActorsOfClass "/Game/Machinations/resources/BP_Resource.BP_Resource_C"))
  (Utilities|Array|SetArrayElem (Variables|/Game/Machinations/resources/BP_Resource.BP_Resource_C|GetData_Resources (Utilities|Array|Get(acopy) _outactors)) 0 (Utilities|Struct|MakeData_Resources "None" 0 (+ (.InInventory (Utilities|Struct|BreakData_Resources (Utilities|Array|Get(acopy) (Variables|/Game/Machinations/resources/BP_Resource.BP_Resource_C|GetData_Resources (Utilities|Array|Get(acopy) _outactors)) (Variables|Default|GetSurvivorCode)))) 1) 0))
  (Variables|Default|SetItHasSurvivor false)
  (return))